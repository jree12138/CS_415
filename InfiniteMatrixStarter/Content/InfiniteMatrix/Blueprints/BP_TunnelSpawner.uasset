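; Spawner for an endless tunnel game that builds BP_Tunnel segments and fills them with Boom hazards, heals and a star.
; On BeginPlay it clears existing tunnels, chains starting segments from the player's location, then resets health, score and level.
; SpawnTunnelAtSpawnPoint extends the furthest tunnel and raises the player's level and score.
; Boom and heal counts grow with level by square and fourth roots, spaced along X with random sine/cosine Y/Z offsets.
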(event `self.ReceiveBeginPlay`
  (`self.SpawnInitialTunnel`))

(fn `spawnboom`
  (params (number :type Integer) (spawnlocation :type "Vector Structure"))
  (bind _returnvalue (`KismetMathLibrary.RandomFloatInRange` 0.0 360.0))
  (bind _returnvalue_2 (- (`self.tunnel radius`) 50.0))
  ;[1 1 1] radomly generate ball in the tunnel
  (for _index (range 1 (+ number 1))
    (`|SpawnActorFromClass` "/Game/InfiniteMatrix/UI/bloodUI/boom.boom_C" (`KismetMathLibrary.MakeTransform` (`KismetMathLibrary.MakeVector` (+ (+ (* _index (/ (- (`self.tunnel long`) 800.0) number)) 200.0) (.x spawnlocation)) (* (`KismetMathLibrary.DegSin` _returnvalue) _returnvalue_2) (* _returnvalue_2 (`KismetMathLibrary.DegCos` _returnvalue))) (struct) (50.0 50.0 50.0)) "Undefined" "MultiplyWithRoot" null null)))

(fn `spawnheal`
  (params (number :type Integer) (spawnlocation :type "Vector Structure"))
  (bind _returnvalue (`KismetMathLibrary.RandomFloatInRange` 0.0 360.0))
  (bind _returnvalue_2 (- (`self.tunnel radius`) 50.0))
  (for _index (range 1 (+ number 1))
    (`|SpawnActorFromClass` "/Game/InfiniteMatrix/UI/bloodUI/heal.heal_C" (`KismetMathLibrary.MakeTransform` (`KismetMathLibrary.MakeVector` (+ (+ (* _index (/ (- (`self.tunnel long`) 800.0) number)) 200.0) (.x spawnlocation)) (* (`KismetMathLibrary.DegSin` _returnvalue) _returnvalue_2) (* _returnvalue_2 (`KismetMathLibrary.DegCos` _returnvalue)))) "Undefined" "MultiplyWithRoot" null null)))

(fn `SpawnInitialTunnel`
  (bind _returnvalue (`GameplayStatics.GetPlayerPawn` 0))
  (`|ExecutionSequence`
    (:`then_0`
      (bind _outactors (`GameplayStatics.GetAllActorsOfClass` "/Game/InfiniteMatrix/Blueprints/BP_Tunnel.BP_Tunnel_C"))
      (for _array_element _outactors
        (`self.K2_DestroyActor` _array_element)))
    (:`then_1`
      (for _ (range 3)
        (`/Engine/EditorBlueprintResources/StandardMacros.IsValid` (`self.FurtherestTunnel`)
          (:`Is Valid`
            (`self.SpawnTunnelAtSpawnPoint`))
          (:`Is Not Valid`
            (`self.SpawnTunne` (`self.K2_GetActorLocation` _returnvalue))))))
    (:`then_2`
      (bind _asbp_player (cast `/Game/InfiniteMatrix/Blueprints/BP_Player` _returnvalue))
      (set `/Game/InfiniteMatrix/Blueprints/BP_Player.CurrentBlood` 100.0 _asbp_player)
      (set `/Game/InfiniteMatrix/Blueprints/BP_Player.TotalBlood` 100.0 _asbp_player))
    (:`then_3`
      (set `/Game/InfiniteMatrix/Blueprints/BP_Player.score` 0 _asbp_player)
      (set `/Game/InfiniteMatrix/Blueprints/BP_Player.level` 0 _asbp_player))))

(fn `spawnstar`
  (params (number :type Integer) (spawnlocation :type "Vector Structure"))
  (bind _returnvalue (`KismetMathLibrary.RandomFloatInRange` 0.0 360.0))
  (bind _returnvalue_2 (- (`self.tunnel radius`) 50.0))
  (for _index (range 1 (+ number 1))
    (`|SpawnActorFromClass` "/Game/InfiniteMatrix/UI/bloodUI/star.star_C" (`KismetMathLibrary.MakeTransform` (`KismetMathLibrary.MakeVector` (+ (+ (* _index (/ (- (`self.tunnel long`) 800.0) number)) 200.0) (.x spawnlocation)) (* (`KismetMathLibrary.DegSin` _returnvalue) _returnvalue_2) (* _returnvalue_2 (`KismetMathLibrary.DegCos` _returnvalue)))) "Undefined" "MultiplyWithRoot" null null)))

(fn `SpawnTunne`
  (params (SpawnLocation :type "Vector Structure"))
  (`|ExecutionSequence`
    (:`then_0`
      ;[1 1 1] new tunnel
      (bind _returnvalue (`|SpawnActorFromClass` "/Game/InfiniteMatrix/Blueprints/BP_Tunnel.BP_Tunnel_C" (`KismetMathLibrary.MakeTransform` SpawnLocation) "Undefined" "MultiplyWithRoot" null null))
      (bind _output_get (set `self.FurtherestTunnel` _returnvalue))
      (set `/Game/InfiniteMatrix/Blueprints/BP_Tunnel.TunnelSpawner` self _output_get)
      (`/Game/InfiniteMatrix/Blueprints/BP_Tunnel.RandomizeWall` _output_get))
    (:`then_1`
      ;[1 1 1] generate enemy;  the number of the enemy follows the  a sqrt funtion
      (bind _asbp_player (cast `/Game/InfiniteMatrix/Blueprints/BP_Player` (`GameplayStatics.GetPlayerPawn` 0)))
      (`self.spawnboom` (`KismetMathLibrary.FTrunc` (+ (`KismetMathLibrary.Sqrt` (`KismetMathLibrary.Conv_IntToDouble` (`/Game/InfiniteMatrix/Blueprints/BP_Player.level` _asbp_player))) 2.0)) SpawnLocation))
    (:`then_2`
      ;[1 1 1] generate the healing point;     using another funciton
      (bind _asbp_player_2 (cast `/Game/InfiniteMatrix/Blueprints/BP_Player` (`GameplayStatics.GetPlayerPawn` 0)))
      (`self.spawnheal` (`KismetMathLibrary.FTrunc` (`KismetMathLibrary.Sqrt` (`KismetMathLibrary.Sqrt` (`KismetMathLibrary.Conv_IntToDouble` (`/Game/InfiniteMatrix/Blueprints/BP_Player.level` _asbp_player_2))))) SpawnLocation))
    (:`then_3`
      (`self.spawnstar` 1 SpawnLocation))))

(fn `SpawnTunnelAtSpawnPoint`
  (`|ExecutionSequence`
    (:`then_0`
      (`self.SpawnTunne` (`SceneComponent.K2_GetComponentLocation` (`/Game/InfiniteMatrix/Blueprints/BP_Tunnel.SpawnPoint` (`self.FurtherestTunnel`)))))
    (:`then_1`
      ;[1 1 1] level reward
      (bind _asbp_player (cast `/Game/InfiniteMatrix/Blueprints/BP_Player` (`GameplayStatics.GetPlayerPawn` 0)))
      (bind _output_get (set `/Game/InfiniteMatrix/Blueprints/BP_Player.level` (+ (`/Game/InfiniteMatrix/Blueprints/BP_Player.level` _asbp_player) 1) _asbp_player))
      (set `/Game/InfiniteMatrix/Blueprints/BP_Player.score` (+ (* _output_get 100) (`/Game/InfiniteMatrix/Blueprints/BP_Player.score` _asbp_player)) _asbp_player))))

(fn `UserConstructionScript`)